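; BP_ISMActor is a debug and test actor for manually driving the Mass traffic simulation and traffic light subsystems.
; Events and functions forward to TrafficSimSubsystem to initialize it, spawn or delete Mass vehicle entities on a target lane, and print that lane's vehicles and links.
; Others call TrafficLightSubsystem to build intersection data from a tag filter, look up an intersection, and set or debug-draw open lanes by zone index.
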(event `Test`
  (`TrafficSimSubsystem.SpawnMassEntities` (subsystem `TrafficSimSubsystem`) 30 (`self.Target Lane`) (`self.Entity Config Asset`)))

(event `Delete`
  (`TrafficSimSubsystem.DeleteMassEntities` (subsystem `TrafficSimSubsystem`) (`self.Target Lane`)))

(event `PrintArray`
  (`TrafficSimSubsystem.PrintLaneVehicles` (subsystem `TrafficSimSubsystem`) (`self.Target Lane`)))

(event `PrintLinks`
  (`TrafficSimSubsystem.PrintLaneLinks` (subsystem `TrafficSimSubsystem`) (`self.Target Lane`)))

(event `BuildIntersec`
  (`TrafficLightSubsystem.BuildIntersectionsData` (subsystem `TrafficLightSubsystem`) "/TrafficSIm/MassTraffic/DA_TagFilter.DA_TagFilter"))

(fn `DrawOpenLanes`
  (`TrafficLightSubsystem.DebugDrawState` (subsystem `TrafficLightSubsystem`) (`self.Zone Index`) 5.0))

(fn `InitTraffisSubsystem`
  (`TrafficSimSubsystem.InitializeManual` (subsystem `TrafficSimSubsystem`)))

(fn `PrintIntersecData`
  (`TrafficLightSubsystem.LookUpIntersection` (subsystem `TrafficLightSubsystem`) (`self.Zone Index`)))

(fn `SetOpenLanes`
  (`TrafficLightSubsystem.SetOpenLanes` (subsystem `TrafficLightSubsystem`) (`self.Zone Index`) (`self.Side Index`) (`self.Turn Type`) (`self.Reset`)))

(fn `UserConstructionScript`)