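; High-resolution vehicle actor for the MassTraffic simulation, with support for being selected.
; Selected looks up the actor's vehicle ID in the traffic sim subsystem, logs it, applies the selection visuals and returns the ID.
; SelectedState toggles the ring circle component and the static mesh's custom depth rendering together.
; The Hitted event is an empty stub.
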(event `Hitted`)

(fn `Selected`
  (params (bEnable :type Boolean))
  (returns (VehID :type Name))
  (bind _returnvalue (`TrafficSimSubsystem.GetVehIDFromActor` (subsystem `TrafficSimSubsystem`) self))
  (`DimensioBPLibrary.PrintLog` (`KismetStringLibrary.Conv_NameToString` _returnvalue) false)
  (`self.SelectedState` bEnable)
  (return _returnvalue))

(fn `SelectedState`
  (params (bNewVisibility :type Boolean))
  (`SceneComponent.SetVisibility` (`self.BPC_RingsOfPower_Circle1`) bNewVisibility false)
  (`PrimitiveComponent.SetRenderCustomDepth` (`self.StaticMesh`) bNewVisibility))

(fn `UserConstructionScript`)