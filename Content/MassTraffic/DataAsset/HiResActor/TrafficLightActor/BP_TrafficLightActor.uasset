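; Traffic light actor for a MassTraffic junction, showing the signal state supplied by TrafficLightSubsystem.
; After a one-tick delay it fetches controlled lanes, averages positions per lane group and spawns one light widget per group.
; Tick polls phase and time left to update the widgets, turning green to yellow under five seconds.
; Debug mode adds a phase clock and instanced-mesh lane markers, and is the only path that updates CurPhase.
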(event `self.ReceiveBeginPlay`
  (bind _asui_traffic_light (cast `/TrafficSIm/MassTraffic/DataAsset/HiResActor/TrafficLightActor/UI_TrafficLight` (`WidgetComponent.GetUserWidgetObject` (`self.Widget`))))
  (bind _output_get (set `self.As UI Traffic Light` _asui_traffic_light))
  (`Widget.SetVisibility` _output_get "Collapsed")
  (set `self.TickEnable` false)
  (`KismetSystemLibrary.DelayUntilNextTick`)
  (bind (_ctllanes _phasetoctllanes _ctllaneinfors) (`TrafficLightSubsystem.GetCrossPhaseCtlLanes` (subsystem `TrafficLightSubsystem`) self))
  (set `self.Ctl Lanes` _ctllanes)
  (set `self.Phase to Ctl Lanes` _phasetoctllanes)
  (bind _output_get_2 (set `self.Ctl Lane Infors` _ctllaneinfors))
  (`|ExecutionSequence`
    (:`then_0`
      (`self.SetActorTickEnabled` true)
      (set `self.TickEnable` true))
    (:`then_1`
      (`self.GenTrafficLightsGroup` _output_get_2))
    (:`then_2`
      (if (`self.Debug`)
        (`self.InitLaneStatus`)
        (`SceneComponent.SetVisibility` (`self.InstancedStaticMesh`) false false)))))

(event `self.ReceiveTick`
  (params (DeltaSeconds :type "Float (single-precision)"))
  (if (`self.TickEnable`)
    (bind (_phase _lefttime) (`TrafficLightSubsystem.GetCrossPhaseState` (subsystem `TrafficLightSubsystem`) self))
    (`|ExecutionSequence`
      (:`then_0`
        ;[0.226 0.226 0.226] DebugPhaseUI
        (if (`self.Debug`)
          (`/TrafficSIm/MassTraffic/DataAsset/HiResActor/TrafficLightActor/UI_TrafficLight.UpdateDisplay` (`self.As UI Traffic Light`) _phase (`KismetMathLibrary.FCeil` _lefttime))))
      (:`then_1`
        (if (!= _phase (`self.CurPhase`))
          (`self.UpdateTrafficLightsPhase` _phase)
          (set `self.YellowPhase` true)
          ;[0.126 0.126 0.126] DebugPhaseCtlLanes
          (if (`self.Debug`)
            (`self.DebugOpenedLane` _phase))))
      (:`then_2`
        ;[1 0.9206 0.09423] Change Green to Yellow at  5 seconds Left
        (if (and (< _lefttime 5.0) (`self.YellowPhase`))
          (set `self.YellowPhase` false)
          (bind _values (`BlueprintMapLibrary.Map_Values` (`self.TrafficLightsGroup`)))
          (for _array_element _values
            (`/TrafficSIm/MassTraffic/DataAsset/HiResActor/TrafficLightActor/UI_TrafficLights.GreenToYellow` _array_element)))))))

(event `DebugLightPhase`
  (bind _isa (`/Engine/EditorBlueprintResources/StandardMacros.FlipFlop`)
    (:`A`
      _)
    (:`B`
      _))
  (set `self.Debug` _isa))

(fn `ClearLaneStatus`
  (`InstancedStaticMeshComponent.ClearInstances` (`self.InstancedStaticMesh`)))

(fn `Debug Lane Infor`
  (locals (PhaseTurnTypes :type String))
  (bind _keys (`BlueprintMapLibrary.Map_Keys` (`self.Ctl Lane Infors`)))
  (for _array_element _keys
    (set `local.PhaseTurnTypes` "")
    (`|ExecutionSequence`
      (:`then_0`
        (bind _value (`BlueprintMapLibrary.Map_Find` (`self.Ctl Lane Infors`) _array_element))
        (bind (_lanetransform _lanesectid _roadid _lanegroup _phaseturntype) (break `CtlLaneInfor` _value))
        (bind _keys_2 (`BlueprintMapLibrary.Map_Keys` _phaseturntype))
        (for _array_element_2 _keys_2
          (set `local.PhaseTurnTypes` (`KismetStringLibrary.Concat_StrStr` (`local.PhaseTurnTypes`) ";" (`KismetStringLibrary.Concat_StrStr` (`KismetStringLibrary.Conv_NameToString` _array_element_2) "-->" (`KismetStringLibrary.Conv_NameToString` (`BlueprintMapLibrary.Map_Find` _phaseturntype _array_element_2)))))))
      (:`then_1`
        (bind (_lanetransform_2 _lanesectid_2 _roadid_2 _lanegroup_2) (break `CtlLaneInfor` _value))
        (`DimensioBPLibrary.PrintLog` (`KismetTextLibrary.Conv_TextToString` (`|FormatText` "Position:{Pos},LaneID:{LID},RoadID:{RID},GroupID:{GID},TurnType:{TurnType}" (`KismetStringLibrary.Conv_VectorToString` (.location _lanetransform_2)) _lanesectid_2 _roadid_2 _lanegroup_2 (`local.PhaseTurnTypes`))))))))

(fn `DebugOpenedLane`
  (params (InputPin :type Name))
  (`|ExecutionSequence`
    (:`then_0`
      (if (== (`self.CurPhase`) "None")
        (`SceneComponent.SetVisibility` (`self.InstancedStaticMesh`) true false)))
    (:`then_1`
      (bind _output_get (set `self.CurPhase` InputPin))
      (if (!= _output_get "None")
        (`self.PhaseToCtlLane` (`self.CurPhase`))
        (else
          (`SceneComponent.SetVisibility` (`self.InstancedStaticMesh`) false false))))))

(fn `DewbugDraw`
  (bind _keys (`BlueprintMapLibrary.Map_Keys` (`self.Ctl Lanes`)))
  (for _array_element _keys
    (bind _location (.location (`BlueprintMapLibrary.Map_Find` (`self.Ctl Lanes`) _array_element)))
    (`KismetSystemLibrary.DrawDebugArrow` _location (+ _location (* (`KismetMathLibrary.GetForwardVector` (.rotation (`BlueprintMapLibrary.Map_Find` (`self.Ctl Lanes`) _array_element))) 500.0)) 100.0 (struct :`R` 1.0 :`G` 0.110968 :`A` 1.0) 15.0 10.0)
    (`DimensioBPLibrary.PrintLog` (`KismetStringLibrary.Conv_IntToString` _array_element))))

(fn `DynamicScaleLight`
  (locals (NewScale :type "Float (single-precision)" :default 0.0))
  (bind ((`Location_5_1CF6D8A9488BFFD43BEB4B875EF51389` _location) (`ZoomLength_12_8E0D2871499666D4FF35149848BFC83C` _zoomlength)) (break `/Dimensio/DirectionDepartment/S_CameraPosture` (`/Dimensio/DirectionDepartment/BP_PawnManager.GetCurrentPosture` (`/Dimensio/GamePlay/GM_Getter/BPFL_GM_Getter.GMGetPawnManager`))))
  (bind _returnvalue (+ _zoomlength (`KismetMathLibrary.Vector_Distance` _location (`self.K2_GetActorLocation`))))
  (if (!= _returnvalue (`self.DistToCam`))
    (set `self.DistToCam` _returnvalue)
    (set `local.NewScale` (`CurveFloat.GetFloatValue` (`self.C_DistToScale`) (`self.DistToCam`)))
    (bind _values (`BlueprintMapLibrary.Map_Values` (`self.TrafficLightsGroup`)))
    (for _array_element _values
      (`/TrafficSIm/MassTraffic/DataAsset/HiResActor/TrafficLightActor/UI_TrafficLights.DynamicScale` _array_element (`local.NewScale`)))))

(fn `GenTrafficLightsGroup`
  (params (LaneInfo :type "Map of Name to CtlLaneInfor Structure"))
  (locals (GroupLanes :type "Map of Integer to Object Object Reference") (GroupLocations :type "Map of Integer to Transform Structure"))
  (bind _returnvalue (`self.GetTransform`))
  (bind _grouplanes (`local.GroupLanes`))
  (bind _grouplocations (`local.GroupLocations`))
  (bind _grouplocations_2 (`local.GroupLocations`))
  (bind _grouplocations_3 (`local.GroupLocations`))
  (bind _laneinfo (`local.LaneInfo`))
  (`|ExecutionSequence`
    (:`then_0`
      ;[1 1 1] Group Location Avg
      (bind _keys (`BlueprintMapLibrary.Map_Keys` LaneInfo))
      (for _array_element _keys
        (`|ExecutionSequence`
          (:`then_0`
            (bind (_lanetransform _lanesectid _roadid _lanegroup) (break `CtlLaneInfor` (`BlueprintMapLibrary.Map_Find` LaneInfo _array_element)))
            (bind (_value _returnvalue_2) (`BlueprintMapLibrary.Map_Find` _grouplanes _lanegroup))
            (if _returnvalue_2
              (`BlueprintMapLibrary.Map_Add` _grouplanes _lanegroup (+ _value 1))
              (else
                (`BlueprintMapLibrary.Map_Add` _grouplanes _lanegroup 1))))
          (:`then_1`
            (bind (_value_2 _returnvalue_3) (`BlueprintMapLibrary.Map_Find` _grouplocations _lanegroup))
            (if _returnvalue_3
              (`BlueprintMapLibrary.Map_Add` _grouplocations _lanegroup (`KismetMathLibrary.MakeTransform` (+ (.location _value_2) (.location _lanetransform)) (.rotation _value_2)))
              (else
                (`BlueprintMapLibrary.Map_Add` _grouplocations _lanegroup _lanetransform))))))
      (bind _keys_2 (`BlueprintMapLibrary.Map_Keys` _grouplocations_2))
      (for _array_element_2 _keys_2
        (`BlueprintMapLibrary.Map_Add` (`local.GroupLocations`) _array_element_2 (`KismetMathLibrary.MakeTransform` (/ (.location (`BlueprintMapLibrary.Map_Find` _grouplocations_2 _array_element_2)) (`KismetMathLibrary.Conv_IntToDouble` (`BlueprintMapLibrary.Map_Find` (`local.GroupLanes`) _array_element_2))) (.rotation (`BlueprintMapLibrary.Map_Find` _grouplocations_2 _array_element_2))))))
    (:`then_1`
      ;[1 1 1] Spawn the TrafficLighs Widget
      (`|ExecutionSequence`
        (:`then_0`
          (bind _keys_3 (`BlueprintMapLibrary.Map_Keys` _grouplocations_3))
          (for _array_element_3 _keys_3
            (bind _returnvalue_4 (`KismetMathLibrary.InverseTransformRotation` _returnvalue (.rotation (`BlueprintMapLibrary.Map_Find` _grouplocations_3 _array_element_3))))
            (bind _returnvalue_5 (`AddComponent|NODE_AddWidgetComponent-0` :`RelativeTransform` (`KismetMathLibrary.MakeTransform` (+ (`KismetMathLibrary.InverseTransformLocation` _returnvalue (.location (`BlueprintMapLibrary.Map_Find` _grouplocations_3 _array_element_3))) (0.0 0.0 500.0) (* (`KismetMathLibrary.GetForwardVector` _returnvalue_4) 400.0)) (`KismetMathLibrary.MakeRotator` (.roll _returnvalue_4) (.pitch _returnvalue_4) (+ (.yaw _returnvalue_4) 180.0)) (0.5 0.5 0.5))))
            (bind _asui_traffic_lights (cast `/TrafficSIm/MassTraffic/DataAsset/HiResActor/TrafficLightActor/UI_TrafficLights` (`WidgetComponent.GetUserWidgetObject` _returnvalue_5)))
            (`BlueprintMapLibrary.Map_Add` (`self.TrafficLightsGroup`) _array_element_3 _asui_traffic_lights)))
        (:`then_1`
          (bind _keys_4 (`BlueprintMapLibrary.Map_Keys` _laneinfo))
          (for _array_element_4 _keys_4
            (bind (_lanetransform_2 _lanesectid_2 _roadid_2 _lanegroup_2 _phaseturntype) (break `CtlLaneInfor` (`BlueprintMapLibrary.Map_Find` _laneinfo _array_element_4)))
            (bind (_value_3 _returnvalue_6) (`BlueprintMapLibrary.Map_Find` (`self.TrafficLightsGroup`) _lanegroup_2))
            (if _returnvalue_6
              (`/TrafficSIm/MassTraffic/DataAsset/HiResActor/TrafficLightActor/UI_TrafficLights.AddPhaseTurnsForLane` _value_3 _phaseturntype))))
        (:`then_2`
          (`self.UpdateTrafficLightsPhase` "None"))))))

(fn `InitLaneStatus`
  (`InstancedStaticMeshComponent.ClearInstances` (`self.InstancedStaticMesh`))
  (bind _keys (`BlueprintMapLibrary.Map_Keys` (`self.Ctl Lanes`)))
  (for _array_element _keys
    (bind _rotation (.rotation (`BlueprintMapLibrary.Map_Find` (`self.Ctl Lanes`) _array_element)))
    (bind _returnvalue (`InstancedStaticMeshComponent.AddInstance` (`self.InstancedStaticMesh`) (`KismetMathLibrary.MakeTransform` (+ (.location (`BlueprintMapLibrary.Map_Find` (`self.Ctl Lanes`) _array_element)) (* (`KismetMathLibrary.GetForwardVector` _rotation) 500.0)) (`KismetMathLibrary.MakeRotator` (.roll _rotation) (.pitch _rotation) (+ (.yaw _rotation) 90.0)) (4.5 4.5 1.0)) true))
    (`BlueprintMapLibrary.Map_Add` (`self.CtlToISMIndex`) _array_element _returnvalue)))

(fn `PhaseToCtlLane`
  (params (Phase :type Name))
  (`|ExecutionSequence`
    (:`then_0`
      (for _index (range (`InstancedStaticMeshComponent.GetInstanceCount` (`self.InstancedStaticMesh`)))
        (`InstancedStaticMeshComponent.SetCustomDataValue` (`self.InstancedStaticMesh`) _index 0 0.0 true)))
    (:`then_2`
      (for _array_element (`.IntArray` (break `ArrayInt` (`BlueprintMapLibrary.Map_Find` (`self.Phase to Ctl Lanes`) Phase)))
        (`InstancedStaticMeshComponent.SetCustomDataValue` (`self.InstancedStaticMesh`) (`BlueprintMapLibrary.Map_Find` (`self.CtlToISMIndex`) _array_element) 0 1.0 true)))))

(fn `Test`
  (for _index (range (`InstancedStaticMeshComponent.GetInstanceCount` (`self.InstancedStaticMesh`)))
    (bind _returnvalue (`InstancedStaticMeshComponent.SetCustomDataValue` (`self.InstancedStaticMesh`) _index 0 1.0 true))
    (`DimensioBPLibrary.PrintLog` (`KismetStringLibrary.Conv_BoolToString` _returnvalue))))

(fn `TestPhase`
  (`SceneComponent.SetVisibility` (`self.InstancedStaticMesh`) true false)
  (`self.PhaseToCtlLane` (`self.DebugPhase`)))

(fn `UpdateTrafficLightsPhase`
  (params (Phase :type Name))
  (if (!= Phase "None")
    (bind _values (`BlueprintMapLibrary.Map_Values` (`self.TrafficLightsGroup`)))
    (for _array_element _values
      (`Widget.SetVisibility` _array_element "Visible")
      (`/TrafficSIm/MassTraffic/DataAsset/HiResActor/TrafficLightActor/UI_TrafficLights.SetPhase` _array_element Phase))
    (else
      (bind _values_2 (`BlueprintMapLibrary.Map_Values` (`self.TrafficLightsGroup`)))
      (for _array_element_2 _values_2
        (`Widget.SetVisibility` _array_element_2 "Hidden")))))

(fn `UserConstructionScript`)