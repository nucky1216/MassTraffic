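; BP_TrafficLightActor is a high-resolution Mass traffic actor for a traffic light that displays its current phase and countdown on a widget.
; On BeginPlay it caches the UI_TrafficLight object from its widget component and logs the entity-to-actor switch.
; Every tick it queries TrafficLightSubsystem for its crossing phase state and passes the phase and rounded-up remaining time to the widget.
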(event `self.ReceiveBeginPlay`
  (bind _asui_traffic_light (cast `/TrafficSIm/MassTraffic/DataAsset/HiResActor/TrafficLight/UI_TrafficLight` (`WidgetComponent.GetUserWidgetObject` (`self.Widget`))))
  (set `self.As UI Traffic Light` _asui_traffic_light)
  (`DimensioBPLibrary.PrintLog` "Entity to Actor!!"))

(event `self.ReceiveTick`
  (params (DeltaSeconds :type "Float (single-precision)"))
  (bind (_phase _lefttime) (`TrafficLightSubsystem.GetCrossPhaseState` (subsystem `TrafficLightSubsystem`) self))
  (`/TrafficSIm/MassTraffic/DataAsset/HiResActor/TrafficLight/UI_TrafficLight.UpdateDisplay` (`self.As UI Traffic Light`) _phase (`KismetMathLibrary.FCeil` _lefttime)))

(fn `UserConstructionScript`)