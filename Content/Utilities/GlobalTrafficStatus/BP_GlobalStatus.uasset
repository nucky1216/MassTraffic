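; BP_GlobalStatus is an actor that displays global traffic status as a Niagara point cloud placed on Cesium georeferenced coordinates.
; PushPoints converts each DataTable row's coordinates to Unreal positions, adjusting height and adding the numeric row name to Z.
; UpdatePoints feeds the points into the Niagara vector array and resets the system.
; GetGeoRef picks a CesiumGeoreference whose name lacks "_84", and ClearGeoRef releases it.
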(fn `ClearGeoRef`
  (set `self.GeoRef` null))

(fn `GetGeoRef`
  (bind _outactors (`GameplayStatics.GetAllActorsOfClass` "/Script/CesiumRuntime.CesiumGeoreference"))
  (for _array_element _outactors
    (if (not (`KismetStringLibrary.Contains` (`KismetSystemLibrary.GetDisplayName` _array_element) "_84" false true))
      (set `self.GeoRef` _array_element))))

(fn `PushPoints`
  (`KismetArrayLibrary.Array_Clear` (`self.Points`))
  (bind _outrownames (`DataTableFunctionLibrary.GetDataTableRowNames` (`self.DataTable`)))
  (for _array_element _outrownames
    (bind _returnvalue (`|GetDataTableRow` (`self.DataTable`) _array_element)
      (:`then`
        (for _array_element_2 (`.coords` (break `DTRoadGeoStatus` _returnvalue))
          (bind _returnvalue_2 (+ (`CesiumGeoreference.TransformLongitudeLatitudeHeightPositionToUnreal` (`self.GeoRef`) (+ (* _array_element_2 (1.0 1.0 2.0)) (0.0 0.0 1.0))) (`KismetMathLibrary.MakeVector` 0.0 0.0 (`KismetStringLibrary.Conv_StringToDouble` (`KismetStringLibrary.Conv_NameToString` _array_element)))))
          (`KismetArrayLibrary.Array_Add` (`self.Points`) _returnvalue_2)
          (`DimensioBPLibrary.PrintLog` (`KismetStringLibrary.Conv_VectorToString` _returnvalue_2))))))
  (`self.UpdatePoints`))

(fn `UpdatePoints`
  (bind _ns_trafficstatus (`self.NS_TrafficStatus`))
  (`NiagaraDataInterfaceArrayFunctionLibrary.SetNiagaraArrayVector` _ns_trafficstatus "VectorArray" (`self.Points`))
  (`NiagaraComponent.ResetSystem` _ns_trafficstatus))

(fn `UserConstructionScript`)