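; BP_GenZoneShape is a utility actor that generates a ZoneShape actor for ZoneGraph lanes.
; GenZoneShape spawns the shape at its own transform, stores it in the ZoneGraph variable and overwrites its shape component's points with a two-point array.
; The lane profile assignment is disconnected, and PrintZoneInfor is an unfinished stub that loops over points without printing.
; Event graph and construction script are empty.
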(fn `GenZoneShape`
  (locals (ZoneGraph :type "ZoneShape Object Reference") (NewLocalVar :type "ZoneLaneProfileRef Structure"))
  (bind _returnvalue (`|SpawnActorFromClass` "/Script/ZoneGraph.ZoneShape" (`self.GetTransform`) "Undefined" "MultiplyWithRoot" null null))
  (bind _output_get (set `local.ZoneGraph` _returnvalue))
  (set `ZoneShapeComponent.Points` (`|MakeArray` (struct) (struct) :!type "ZoneShapePoint Structure") (`ZoneShape.ShapeComponent` _output_get)))

(fn `PrintZoneInfor`
  (for _ (`ZoneShapeComponent.Points` (`ZoneShape.ShapeComponent` (`self.ZoneShape`)))
    _))

(fn `UserConstructionScript`)