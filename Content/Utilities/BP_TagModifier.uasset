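; BP_TagModifier is a utility actor that bulk-edits tags on ZoneShape actors.
; Its AddCIIETag function finds every ZoneShape with the actor tag "CIIE", combines TagToAdd with the shape component's current tags through AddShapeTag, and writes the result back.
; The event graph and construction script are empty, and a disconnected single-Zone version of the tag edit never runs.
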(fn `Add CIIE Tag`
  (bind _outactors (`GameplayStatics.GetAllActorsOfClassWithTag` "/Script/ZoneGraph.ZoneShape" "CIIE"))
  (for _array_element _outactors
    (bind _shapecomponent (`ZoneShape.ShapeComponent` _array_element))
    (`ZoneShapeComponent.SetTags` _shapecomponent (`BPFLTools.AddShapeTag` (`ZoneShapeComponent.GetTags` _shapecomponent) (`self.TagToAdd`)))))

(fn `UserConstructionScript`)