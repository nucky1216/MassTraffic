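; Data request actor that periodically POSTs JSON to a configured URL to fetch road data for a traffic visualizer.
; A looping timer sends the request, and successful responses are converted with a lane map into a DataTable, then broadcast through DataTableReady.
; TrafficVisualizer view state pauses or resumes polling.
; URL, request body and interval live in a struct exchanged as JSON, and setting it restarts the timer.
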(event `self.ReceiveBeginPlay`
  (`parent.ReceiveBeginPlay`)
  (`self.SetTimer`)
  (add `/TrafficSIm/Data/BP_TrafficVisualizer.OnViewStateChanged` (`self.TrafficVisualizer`) (`|CreateDelegate` :!event `On View State Changed`)))

(fn `Data Table Filled Finished`
  (params (RoadDT :type "DataTable Object Reference"))
  (`self.DataTableReady` RoadDT))

(fn `GetClassProp`
  (returns (ClassProp :type "JsonLibraryObject Structure"))
  (return (`JsonLibraryStructHelperBPLibrary.JsonObject_FromStruct` (`self.Classprop`))))

(fn `Http Response`
  (params (Url :type String) (bSuccess :type Boolean) (Code :type Integer) (Content :type "Array of Byte (by ref)"))
  (`DimensioBPLibrary.PrintLog` (`KismetTextLibrary.Conv_TextToString` (`|FormatText` "Response from :{URL} \nSuccess:{sucess} \nCode:{Code}" Url bSuccess Code)))
  (`|ExecutionSequence`
    (:`then_0`
      (if (== Code 200)
        (`BPFLTools.JsonToDT` Content (`self.Nav Map`) (`|CreateDelegate` :!event `Data Table Filled Finished`))
        (return)))))

(fn `On View State Changed`
  (params (NewState :type "/TrafficSIm/Data/E_ZoomRangeState Enum" :default "NewEnumerator0"))
  (if (`|EnumEquality` NewState "NewEnumerator0")
    (`KismetSystemLibrary.K2_PauseTimerHandle` (`self.TimerHandle`))
    (else
      (`KismetSystemLibrary.K2_UnPauseTimerHandle` (`self.TimerHandle`)))))

(fn `SendRequest`
  (bind (_url _requestjson) (break `/TrafficSIm/Data/S_DataRequest` (`self.Classprop`)))
  (bind _curstate (`/TrafficSIm/Data/BP_TrafficVisualizer.GetViewState` (`self.TrafficVisualizer`)))
  (bind _returnvalue (`ReHttpClientBPFL.SendHttpRequestWithCallback` _url "Post" "json" (`ReHttpClientBPFL.ByteArray_FromString` _requestjson) (`|CreateDelegate` :!event `Http Response`)))
  (`DimensioBPLibrary.PrintLog` (`KismetStringLibrary.Concat_StrStr` "Send Http Request:" (`KismetStringLibrary.Conv_BoolToString` _returnvalue) " with url:" _url))
  (`/Engine/EditorBlueprintResources/StandardMacros.IsValid` (`self.TrafficVisualizer`)
    (:`Is Valid`
      (if (and (`|EnumInequality` _curstate "NewEnumerator1") (`|EnumInequality` _curstate "NewEnumerator2"))
        (`KismetSystemLibrary.K2_PauseTimerHandle` (`self.TimerHandle`))))))

(fn `SetClassProp`
  (params (ClassProp :type "JsonLibraryObject Structure"))
  (returns (ReturnMessage :type "/Dimensio/Communication/Message/S_VO_ReturnMessage Structure"))
  (`JsonLibraryStructHelperBPLibrary.JsonObject_ToStruct` ClassProp (`self.Classprop`))
  (`self.SetTimer`)
  (return))

(fn `SetTimer`
  (bind ((`RequestJson_9_2AEB9F42440B45A043838888067FEC26` _requestjson) (`Duration_8_05368A2B4EB82A86E1F0FF9AC909413E` _duration)) (break `/TrafficSIm/Data/S_DataRequest` (`self.Classprop`)))
  (if (`KismetSystemLibrary.K2_IsValidTimerHandle` (`self.TimerHandle`))
    (`KismetSystemLibrary.K2_ClearAndInvalidateTimerHandle` (`self.TimerHandle`)))
  (if (> (`.Duration_8_05368A2B4EB82A86E1F0FF9AC909413E` (break `/TrafficSIm/Data/S_DataRequest` (`self.Classprop`))) 0.0)
    (bind _returnvalue (`KismetSystemLibrary.K2_SetTimer` null "SendRequest" _duration true (* _duration -1.0)))
    (set `self.TimerHandle` _returnvalue)))

(fn `UserConstructionScript`
  (`parent.UserConstructionScript`))